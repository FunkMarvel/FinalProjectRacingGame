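; BP_CarPawn is a car pawn Blueprint that handles driving visual effects for sharp turns and landings.
; A max-turn event drives the right or left Niagara spark amount from the physics sphere's speed, and a not-max-turn event zeroes both sides.
; A hit-ground event activates an impact particle system.
; The graph holds no movement logic and only reacts to these events.
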(event EventBeginPlay)

(event Collision|EventActorBeginOverlap
  (params (OtherActor :type Actor%20Object%20Reference)))

(event EventTick
  (params (DeltaSeconds :type Float%20%28single-precision%29)))

(event EventMaxTurnBpEvent
  (params (bRightSide :type Boolean))
  (bind _returnvalue (Physics|GetPhysicsLinearVelocity (Variables|Default|GetSphereComp) "None"))
  (if bRightSide
    (Effects|Components|ParticleSystem|SetFloatParameter (Variables|Default|GetNS_Sparkles_Right) "sparkAmmount" (/ (Math|Vector|VectorLength _returnvalue) 1e+01))
    (else
      (Effects|Components|ParticleSystem|SetFloatParameter (Variables|Default|GetNS_Sparkles_Left) "sparkAmmount" (/ (Math|Vector|VectorLength _returnvalue) 1e+01)))))

(event EventNotMaxTurnBpEvent
  (Effects|Components|ParticleSystem|SetFloatParameter (Variables|Default|GetNS_Sparkles_Right) "sparkAmmount" 0.0)
  (Effects|Components|ParticleSystem|SetFloatParameter (Variables|Default|GetNS_Sparkles_Left) "sparkAmmount" 0.0))

(event EventHitGroundBpEvent
  (params (Speed :type Float%20%28single-precision%29))
  (Components|Activation|Activate (Variables|Default|GetHitGroundParticleSystem) false))

(fn ConstructionScript)