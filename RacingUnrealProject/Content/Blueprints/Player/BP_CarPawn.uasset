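; Shark-themed car pawn Blueprint that handles the vehicle's cosmetic feedback, with no movement logic in this graph.
; Turn, speed and ground-hit events drive Niagara sparks scaled by physics velocity, clamped booster sizes, the body AnimBP's speed and an impact particle.
; The grapple component's OpenHead event chains shark head montages from open to fly, or close to idle.
; Entering the Dying state hides both boosters for the dying duration.
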(event OpenHead(PhysicsGrappleComponent)
  (params (bOpen :type Boolean))
  (bind _sharkheadmesh (Variables|Default|GetSharkHeadMesh))
  (if bOpen
    (Animation|Montage|PlayMontage _sharkheadmesh "/Game/Meshes/Shark/NEW/Shark_Head_Open01_Montage.Shark_Head_Open01_Montage"
      (:OnCompleted
        (Animation|Montage|PlayMontage _sharkheadmesh "/Game/Meshes/Shark/NEW/Shark_Head_Fly01_Montage.Shark_Head_Fly01_Montage")))
    (else
      (Animation|Montage|PlayMontage _sharkheadmesh "/Game/Meshes/Shark/NEW/Shark_Head_Close01_Montage.Shark_Head_Close01_Montage"
        (:OnCompleted
          (Animation|Montage|PlayMontage _sharkheadmesh "/Game/Meshes/Shark/NEW/Shark_Head_Idle01_Anim_Montage.Shark_Head_Idle01_Anim_Montage"))))))

(event EventBeginPlay)

(event Collision|EventActorBeginOverlap
  (params (OtherActor :type Actor%20Object%20Reference)))

(event EventTick
  (params (DeltaSeconds :type Float%20%28single-precision%29)))

(event EventMaxTurnBpEvent
  (params (bRightSide :type Boolean))
  (bind _returnvalue (Physics|GetPhysicsLinearVelocity (Variables|Default|GetSphereComp) "None"))
  (if bRightSide
    (Effects|Components|ParticleSystem|SetFloatParameter (Variables|Default|GetNS_Sparkles_Right) "sparkAmmount" (/ (Math|Vector|VectorLength _returnvalue) 69.0))
    (else
      (Effects|Components|ParticleSystem|SetFloatParameter (Variables|Default|GetNS_Sparkles_Left) "sparkAmmount" (/ (Math|Vector|VectorLength _returnvalue) 69.0)))))

(event EventNotMaxTurnBpEvent
  (Effects|Components|ParticleSystem|SetFloatParameter (Variables|Default|GetNS_Sparkles_Right) "sparkAmmount" 0.0)
  (Effects|Components|ParticleSystem|SetFloatParameter (Variables|Default|GetNS_Sparkles_Left) "sparkAmmount" 0.0))

(event EventHitGroundBpEvent
  (params (Speed :type Float%20%28single-precision%29))
  (Components|Activation|Activate (Variables|Default|GetHitGroundParticleSystem) false))

(event EventBPECarSpeed
  (params (Speed :type Float%20%28single-precision%29))
  (bind _returnvalue (* Speed 1.0))
  (bind _returnvalue_2 (* Speed 0.5))
  (bind _ns_boostereffectleft (Variables|Default|GetNS_BoosterEffectLeft))
  (bind _ns_boostereffectright (Variables|Default|GetNS_BoosterEffectRight))
  (bind _returnvalue_3 (Math|Float|Clamp(Float) _returnvalue 0.3 2.0))
  (bind _returnvalue_4 (Math|Float|Clamp(Float) _returnvalue_2 0.3 0.6))
  (Effects|Components|ParticleSystem|SetFloatParameter _ns_boostereffectleft "CoreSize" _returnvalue_4)
  (Effects|Components|ParticleSystem|SetFloatParameter _ns_boostereffectright "CoreSize" _returnvalue_4)
  (Effects|Components|ParticleSystem|SetFloatParameter _ns_boostereffectleft "TailSize" _returnvalue_3)
  (Effects|Components|ParticleSystem|SetFloatParameter _ns_boostereffectright "TailSize" _returnvalue_3)
  (bind _asab_shark_body (Utilities|Casting|CastToAB_SharkBody (Components|SkeletalMesh|GetAnimInstance (Variables|Default|GetSharkBodyMesh))))
  (Variables|/Game/Meshes/Shark/NEW/AB_SharkBody.AB_SharkBody_C|SetSpeed _asab_shark_body (* Speed 7e+01)))

(event EventBPEonEnterNewState
  (params (_NewState :type EVehicleState%20Enum :default "Driving"))
  (switch Utilities|FlowControl|Switch|SwitchonEVehicleState _NewState
    (:Dying
      (Rendering|SetVisibility (Variables|Default|GetNS_BoosterEffectLeft) false false)
      (Utilities|FlowControl|Delay (Variables|Default|GetDyingDuration))
      (Rendering|SetVisibility (Variables|Default|GetNS_BoosterEffectRight) true false))))

(fn ConstructionScript)