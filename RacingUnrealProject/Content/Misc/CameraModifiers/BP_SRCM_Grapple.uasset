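; Camera modifier that, going by its name, adds a screen and field-of-view effect for grappling.
; A curve sampled at the modifier's Alpha drives both outputs, so they blend together.
; The curve value sets the blend weight of fixed post-process intensity overrides and scales an FOV increase, leaving view location and rotation untouched.
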(fn BlueprintModifyPostProcess
  (params (DeltaTime :type Float%20%28single-precision%29))
  (return (Math|Curves|GetFloatValue (Variables|Default|GetCurve) (Variables|Default|GetAlpha)) (Utilities|Struct|MakePostProcessSettings 35.0 1e+02)))

(fn BlueprintModifyCamera
  (params (DeltaTime :type Float%20%28single-precision%29) (ViewLocation :type Vector :default "0, 0, 0") (ViewRotation :type Rotator :default "0, 0, 0") (FOV :type Float%20%28single-precision%29))
  (return ViewLocation ViewRotation (+ FOV (* (Math|Curves|GetFloatValue (Variables|Default|GetCurve) (Variables|Default|GetAlpha)) 3e+01))))